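; BP_DoorLocked is a locked door that the player can remove when carrying a key.
; Box overlap with BP_GabPerso toggles input and opens or closes a gate for the interact action.
; With HasKey set, interacting plays the OpenCloseDoor timeline, whose update clears the key, destroys the door and removes WB_Key and WB_Green widgets.
; The rotation logic is disconnected, so the door vanishes instead of swinging open.
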(event OnComponentBeginOverlap(Box)
  (params (OverlappedComponent :type Primitive%20Component%20Object%20Reference) (OtherActor :type Actor%20Object%20Reference) (OtherComp :type Primitive%20Component%20Object%20Reference) (OtherBodyIndex :type Integer) (bFromSweep :type Boolean) (SweepResult :type Hit%20Result%20Structure%20%28by%20ref%29))
  (bind _asbp_gab_perso (Utilities|Casting|CastToBP_GabPerso OtherActor))
  (Input|EnableInput (Game|GetPlayerController 0))
  (Utilities|FlowControl|Gate true) ; enters at Open
)

(event OnComponentEndOverlap(Box)
  (params (OverlappedComponent :type Primitive%20Component%20Object%20Reference) (OtherActor :type Actor%20Object%20Reference) (OtherComp :type Primitive%20Component%20Object%20Reference) (OtherBodyIndex :type Integer))
  (Utilities|Casting|CastToBP_GabPerso OtherActor)
  (Input|DisableInput (Game|GetPlayerController 0))
  (Utilities|FlowControl|Gate true) ; enters at Close
)

(event Input|EnhancedActionEvents|EnhancedInputActionIA_Interract
  (params (ActionValue :type Boolean) (ElapsedSeconds :type Float%20%28double-precision%29) (TriggeredSeconds :type Float%20%28double-precision%29) (InputAction :type Input%20Action%20Object%20Reference :default "/Game/Anthonin/Door-Key/IA_Interract.IA_Interract"))
  (:Triggered
    ;[0 0.07145 1] Link the TXT "No key" to false
    (if (Variables|/Game/Gabriel/BP_GabPerso.BP_GabPerso_C|GetHasKey? (stale OnComponentBeginOverlap(Box) _asbp_gab_perso))
      (Utilities|FlowControl|Gate true
        (:Exit
          (Utilities|FlowControl|FlipFlop
            (:A
              (Timeline|Open%20/%20Close%20Door Play
                (:Update
                  (Variables|/Game/Gabriel/BP_GabPerso.BP_GabPerso_C|SetHasKey? (stale OnComponentBeginOverlap(Box) _asbp_gab_perso) false)
                  (Actor|DestroyActor)
                  (bind _foundwidgets (Widget|GetAllWidgetsOfClass "/Game/Ewan/UI/WB_Key.WB_Key_C" true))
                  (for _array_element _foundwidgets
                    (Widget|RemovefromParent _array_element)
                    (bind _foundwidgets_2 (Widget|GetAllWidgetsOfClass "/Game/Ewan/UI/WB_Green.WB_Green_C" true))
                    (for _array_element_2 _foundwidgets_2
                      (Widget|RemovefromParent _array_element_2))))))
            (:B
              (Timeline|Open%20/%20Close%20Door Reverse))))))))

(fn ConstructionScript)