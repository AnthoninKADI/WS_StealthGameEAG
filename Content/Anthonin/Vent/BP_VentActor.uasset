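; BP_VentActor is a vent the player can enter and exit, with a timed respawn penalty for staying inside.
; Enter and exit overlaps pass the vent and target location to BP_GabPerso.
; Open/CloseVent swings a pivot via timelines with collision disabled, then toggles InVent and the linked ground's opacity.
; Entering shows WB_Timer and respawns the player if still inside after the delay; the construction script draws a debug trace to that ground.
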(event OnComponentBeginOverlap(EnterCollision)
  (params (OverlappedComponent :type Primitive%20Component%20Object%20Reference) (OtherActor :type Actor%20Object%20Reference) (OtherComp :type Primitive%20Component%20Object%20Reference) (OtherBodyIndex :type Integer) (bFromSweep :type Boolean) (SweepResult :type Hit%20Result%20Structure%20%28by%20ref%29))
  ;[1 1 1] Setting locations for entering the vent
  (if (== OtherActor (Game|GetPlayerCharacter 0))
    (bind _asbp_gab_perso (Utilities|Casting|CastToBP_GabPerso OtherActor))
    (Default|SetVentInfo _asbp_gab_perso true self (Transformation|GetWorldLocation (Variables|Default|GetVent)))))

(event OnComponentEndOverlap(EnterCollision)
  (params (OverlappedComponent :type Primitive%20Component%20Object%20Reference) (OtherActor :type Actor%20Object%20Reference) (OtherComp :type Primitive%20Component%20Object%20Reference) (OtherBodyIndex :type Integer))
  ;[1 1 1] Setting locations for entering the vent
  (if (== OtherActor (Game|GetPlayerCharacter 0))
    (bind _asbp_gab_perso (Utilities|Casting|CastToBP_GabPerso OtherActor))
    (Default|SetVentInfo _asbp_gab_perso false 0 "0, 0, 0")))

(event OnComponentBeginOverlap(ExitCollision)
  (params (OverlappedComponent :type Primitive%20Component%20Object%20Reference) (OtherActor :type Actor%20Object%20Reference) (OtherComp :type Primitive%20Component%20Object%20Reference) (OtherBodyIndex :type Integer) (bFromSweep :type Boolean) (SweepResult :type Hit%20Result%20Structure%20%28by%20ref%29))
  ;[1 1 1] Setting locations for exiting the vent
  (if (== OtherActor (Game|GetPlayerCharacter 0))
    (bind _asbp_gab_perso (Utilities|Casting|CastToBP_GabPerso OtherActor))
    (Default|SetVentInfo _asbp_gab_perso true self (+ (Transformation|GetWorldLocation (Variables|Default|GetVent)) (Math|Vector|MakeVector 0.0 0.0 (Variables|/Script/Engine.CapsuleComponent|GetCapsuleHalfHeight (Variables|/Script/Engine.Character|GetCapsuleComponent _asbp_gab_perso)))))))

(event OnComponentEndOverlap(ExitCollision)
  (params (OverlappedComponent :type Primitive%20Component%20Object%20Reference) (OtherActor :type Actor%20Object%20Reference) (OtherComp :type Primitive%20Component%20Object%20Reference) (OtherBodyIndex :type Integer))
  ;[1 1 1] Setting locations for exiting the vent
  (if (== OtherActor (Game|GetPlayerCharacter 0))
    (bind _asbp_gab_perso (Utilities|Casting|CastToBP_GabPerso OtherActor))
    (Default|SetVentInfo _asbp_gab_perso false 0 "0, 0, 0")))

(event Custom|Open/Close%20Vent
  (bind _vent (Variables|Default|GetVent))
  (bind _vent_2 (Variables|Default|GetVent))
  ;[1 1 1] Open and close the vent using timelines to control rotation of the scene component (act as a pivot). Collision turn off so the player can drop down.
  (if (Variables|/Game/Gabriel/BP_GabPerso.BP_GabPerso_C|GetInVent? (.AsBP%20Gab%20Perso (Utilities|Casting|CastToBP_GabPerso (Game|GetPlayerCharacter 0))))
    (bind _value (Timeline|VentExit Play)
      (:Update
        (Collision|SetCollisionEnabled _vent_2 "NoCollision")
        (Transformation|SetRelativeRotation (Variables|Default|GetScene) (Math|Rotator|MakeRotator 0.0 (Math|Float|Lerp 0.0 9e+01 _value) 0.0) false false))
      (:Finished
        (Collision|SetCollisionEnabled _vent_2 "QueryAndPhysics")
        (bind _asbp_gab_perso (Utilities|Casting|CastToBP_GabPerso (Game|GetPlayerCharacter 0)))
        (Variables|/Game/Gabriel/BP_GabPerso.BP_GabPerso_C|SetInVent? _asbp_gab_perso false)
        (Variables|Default|SetOpacityCheck false)
        (CallFunction|Update)
        (bind _foundwidgets (Widget|GetAllWidgetsOfClass "/Game/Ewan/WB_Timer.WB_Timer_C" true))
        (for _array_element _foundwidgets
          (Widget|RemovefromParent _array_element))))
    (else
      (CallFunction|AlertGuard)
      (bind _value_2 (Timeline|VentEnter Play)
        (:Update
          (Collision|SetCollisionEnabled _vent "NoCollision")
          (Transformation|SetRelativeRotation (Variables|Default|GetScene) (Math|Rotator|MakeRotator 0.0 (Math|Float|Lerp 0.0 9e+01 _value_2) 0.0) false false))
        (:Finished
          (Collision|SetCollisionEnabled _vent "QueryAndPhysics")
          (Variables|/Game/Gabriel/BP_GabPerso.BP_GabPerso_C|SetInVent? (.AsBP%20Gab%20Perso (Utilities|Casting|CastToBP_GabPerso (Game|GetPlayerCharacter 0))) true)
          (Variables|Default|SetOpacityCheck true)
          (CallFunction|Update))))))

(event Custom|Update
  (bind _opacitycheck (Variables|Default|GetOpacityCheck))
  (bind _ref_bp_ground (Variables|Default|GetRef%20BP_Ground))
  (if _opacitycheck
    (Default|Opacity _ref_bp_ground _opacitycheck)
    (else
      (Default|Opacity _ref_bp_ground _opacitycheck))))

(event Custom|AlertGuard
  (bind _returnvalue (Game|GetPlayerCharacter 0))
  ;[1 1 1] Start death Timer - 5sec timer before respawn after entering a vent
  (bind _returnvalue_2 (UserInterface|CreateWidget "/Game/Ewan/WB_Timer.WB_Timer_C" (Game|GetPlayerController 0)))
  (UserInterface|Viewport|AddtoViewport _returnvalue_2 0)
  (Utilities|FlowControl|Delay (Variables|Default|GetTime))
  (if (Variables|/Game/Gabriel/BP_GabPerso.BP_GabPerso_C|GetInVent? (.AsBP%20Gab%20Perso (Utilities|Casting|CastToBP_GabPerso (Game|GetPlayerCharacter 0))))
    (bind _asbp_gab_perso (Utilities|Casting|CastToBP_GabPerso (Game|GetPlayerCharacter 0)))
    (Default|Respawn _asbp_gab_perso)
    (bind _foundwidgets (Widget|GetAllWidgetsOfClass "/Game/Ewan/WB_Timer.WB_Timer_C" true))
    (for _array_element _foundwidgets
      (Widget|RemovefromParent _array_element)
      (if (AI|Components|NavMovement|IsCrouching (Variables|/Script/Engine.Character|GetCharacterMovement _returnvalue))
        (Character|UnCrouch _returnvalue)
        (Variables|/Game/Gabriel/BP_GabPerso.BP_GabPerso_C|SetInVent? (.AsBP%20Gab%20Perso (Utilities|Casting|CastToBP_GabPerso _returnvalue)) false)))))

(fn ConstructionScript
  (Collision|LineTraceByChannel (Transformation|GetWorldLocation (Variables|Default|GetScene self)) (Transformation|GetWorldLocation (Variables|/Game/Anthonin/Vent/BP_GroundTransparent.BP_GroundTransparent_C|GetBillboard (Variables|Default|GetRef%20BP_Ground))) "TraceTypeQuery1" false 0 "ForDuration"))