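; BP_EndGame is an interactable trigger that ends the game for the player character, BP_GabPerso.
; Overlapping its Box enables input and opens a Gate, and leaving disables input and closes it.
; IA_Interract passing the Gate clears all widgets, shows UWBP_EndGame and sets the character's walk speed to zero.
; A final Delay follows with nothing wired after it.
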(event OnComponentBeginOverlap(Box)
  (params (OverlappedComponent :type Primitive%20Component%20Object%20Reference) (OtherActor :type Actor%20Object%20Reference) (OtherComp :type Primitive%20Component%20Object%20Reference) (OtherBodyIndex :type Integer) (bFromSweep :type Boolean) (SweepResult :type Hit%20Result%20Structure%20%28by%20ref%29))
  (Utilities|Casting|CastToBP_GabPerso OtherActor)
  (Input|EnableInput (Game|GetPlayerController 0))
  (Utilities|FlowControl|Gate true) ; enters at Open
)

(event OnComponentEndOverlap(Box)
  (params (OverlappedComponent :type Primitive%20Component%20Object%20Reference) (OtherActor :type Actor%20Object%20Reference) (OtherComp :type Primitive%20Component%20Object%20Reference) (OtherBodyIndex :type Integer))
  (Utilities|Casting|CastToBP_GabPerso OtherActor)
  (Input|DisableInput (Game|GetPlayerController 0))
  (Utilities|FlowControl|Gate true) ; enters at Close
)

(event Input|EnhancedActionEvents|EnhancedInputActionIA_Interract
  (params (ActionValue :type Boolean) (ElapsedSeconds :type Float%20%28double-precision%29) (TriggeredSeconds :type Float%20%28double-precision%29) (InputAction :type Input%20Action%20Object%20Reference :default "/Game/Anthonin/Door-Key/IA_Interract.IA_Interract"))
  (:Triggered
    (Utilities|FlowControl|Gate true
      (:Exit
        (Viewport|RemoveAllWidgets)
        ;[0 0.09849 1] Show EndGame Widget
        (bind _returnvalue (UserInterface|CreateWidget "/Game/Anthonin/EndGame/UWBP_EndGame.UWBP_EndGame_C" (Game|GetPlayerController 0)))
        (UserInterface|Viewport|AddtoViewport _returnvalue 0)
        (Variables|/Script/Engine.CharacterMovementComponent|SetMaxWalkSpeed (Variables|/Script/Engine.Character|GetCharacterMovement (.AsBP%20Gab%20Perso (Utilities|Casting|CastToBP_GabPerso (Game|GetPlayerCharacter 0)))) 0.0)
        (Utilities|FlowControl|Delay 4.0)))))

(fn ConstructionScript)