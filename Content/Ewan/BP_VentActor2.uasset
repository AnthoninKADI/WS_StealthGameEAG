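; A vent actor that the player character BP_GabPerso can enter and exit through a swinging cover.
; Enter and exit overlap volumes pass the player vent availability and a target location, raised by capsule half-height for exiting.
; Open/CloseVent picks a timeline from InVent, pitches a pivot with collision off, then flips InVent.
; It also calls AlertGuard, which respawns the player after a delay; ground material-toggle logic is unconnected.
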(event OnComponentBeginOverlap(EnterCollision)
  (params (OverlappedComponent :type Primitive%20Component%20Object%20Reference) (OtherActor :type Actor%20Object%20Reference) (OtherComp :type Primitive%20Component%20Object%20Reference) (OtherBodyIndex :type Integer) (bFromSweep :type Boolean) (SweepResult :type Hit%20Result%20Structure%20%28by%20ref%29))
  ;[1 1 1] Setting locations for entering the vent
  (if (== OtherActor (Game|GetPlayerCharacter 0))
    (bind _asbp_gab_perso (Utilities|Casting|CastToBP_GabPerso OtherActor))
    (Default|SetVentInfo _asbp_gab_perso true self (Transformation|GetWorldLocation (Variables|Default|GetVent)))))

(event OnComponentEndOverlap(EnterCollision)
  (params (OverlappedComponent :type Primitive%20Component%20Object%20Reference) (OtherActor :type Actor%20Object%20Reference) (OtherComp :type Primitive%20Component%20Object%20Reference) (OtherBodyIndex :type Integer))
  ;[1 1 1] Setting locations for entering the vent
  (if (== OtherActor (Game|GetPlayerCharacter 0))
    (bind _asbp_gab_perso (Utilities|Casting|CastToBP_GabPerso OtherActor))
    (Default|SetVentInfo _asbp_gab_perso false 0 "0, 0, 0")))

(event OnComponentBeginOverlap(ExitCollision)
  (params (OverlappedComponent :type Primitive%20Component%20Object%20Reference) (OtherActor :type Actor%20Object%20Reference) (OtherComp :type Primitive%20Component%20Object%20Reference) (OtherBodyIndex :type Integer) (bFromSweep :type Boolean) (SweepResult :type Hit%20Result%20Structure%20%28by%20ref%29))
  ;[1 1 1] Setting locations for exiting the vent
  (if (== OtherActor (Game|GetPlayerCharacter 0))
    (bind _asbp_gab_perso (Utilities|Casting|CastToBP_GabPerso OtherActor))
    (Default|SetVentInfo _asbp_gab_perso true self (+ (Transformation|GetWorldLocation (Variables|Default|GetVent)) (Math|Vector|MakeVector 0.0 0.0 (Variables|/Script/Engine.CapsuleComponent|GetCapsuleHalfHeight (Variables|/Script/Engine.Character|GetCapsuleComponent _asbp_gab_perso)))))))

(event OnComponentEndOverlap(ExitCollision)
  (params (OverlappedComponent :type Primitive%20Component%20Object%20Reference) (OtherActor :type Actor%20Object%20Reference) (OtherComp :type Primitive%20Component%20Object%20Reference) (OtherBodyIndex :type Integer))
  ;[1 1 1] Setting locations for exiting the vent
  (if (== OtherActor (Game|GetPlayerCharacter 0))
    (bind _asbp_gab_perso (Utilities|Casting|CastToBP_GabPerso OtherActor))
    (Default|SetVentInfo _asbp_gab_perso false 0 "0, 0, 0")))

(event Custom|Open/Close%20Vent
  (bind _vent (Variables|Default|GetVent))
  (bind _vent_2 (Variables|Default|GetVent))
  ;[1 1 1] Open and close the vent using timelines to control rotation of the scene component (act as a pivot). Collision turn off so the player can drop down.
  (Utilities|FlowControl|Sequence
    (:then_0
      (if (Variables|/Game/Gabriel/BP_GabPerso.BP_GabPerso_C|GetInVent? (.AsBP%20Gab%20Perso (Utilities|Casting|CastToBP_GabPerso (Game|GetPlayerCharacter 0))))
        (bind _value (Timeline|VentExit Play)
          (:Update
            (Collision|SetCollisionEnabled _vent_2 "NoCollision")
            (Transformation|SetRelativeRotation (Variables|Default|GetScene) (Math|Rotator|MakeRotator 0.0 (Math|Float|Lerp 0.0 9e+01 _value) 0.0) false false))
          (:Finished
            (Collision|SetCollisionEnabled _vent_2 "QueryAndPhysics")
            (bind _asbp_gab_perso (Utilities|Casting|CastToBP_GabPerso (Game|GetPlayerCharacter 0)))
            (Variables|/Game/Gabriel/BP_GabPerso.BP_GabPerso_C|SetInVent? _asbp_gab_perso false)))
        (else
          (bind _value_2 (Timeline|VentEnter Play)
            (:Update
              (Collision|SetCollisionEnabled _vent "NoCollision")
              (Transformation|SetRelativeRotation (Variables|Default|GetScene) (Math|Rotator|MakeRotator 0.0 (Math|Float|Lerp 0.0 9e+01 _value_2) 0.0) false false))
            (:Finished
              (Collision|SetCollisionEnabled _vent "QueryAndPhysics")
              (Variables|/Game/Gabriel/BP_GabPerso.BP_GabPerso_C|SetInVent? (.AsBP%20Gab%20Perso (Utilities|Casting|CastToBP_GabPerso (Game|GetPlayerCharacter 0))) true))))))
    (:then_1
      (CallFunction|AlertGuard))))

(event Custom|AlertGuard
  (Utilities|FlowControl|Delay 2.0)
  (bind _asbp_gab_perso (Utilities|Casting|CastToBP_GabPerso (Game|GetPlayerCharacter 0)))
  (Default|Respawn _asbp_gab_perso))

(event Input|KeyboardEvents|E
  (params (Key :type Key%20Structure :default "None")))

(fn ConstructionScript)