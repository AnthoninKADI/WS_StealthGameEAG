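; Guard character that catches the player on sight and sends them back to respawn.
; BeginPlay matches a spotlight cone and the PawnSensing peripheral angle to one VisionAngle, so the light shows the detection area.
; Seeing the player freezes their movement and shows a red widget, then after a delay respawns them, clears the widgets and restores speed.
; A separate VentCheck event respawns the player immediately if they are in a vent.
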(event OnSeePawn(PawnSensing)
  (params (Pawn :type Pawn%20Object%20Reference))
  (bind _returnvalue (Game|Player|GetPlayerPawn 0))
  (if (== Pawn _returnvalue)
    (Variables|Default|SetIsSeeing true)
    (bind _asbp_gab_perso (Utilities|Casting|CastToBP_GabPerso _returnvalue))
    (Variables|/Script/Engine.CharacterMovementComponent|SetMaxWalkSpeed (Variables|/Script/Engine.Character|GetCharacterMovement _asbp_gab_perso) 0.0)
    (bind _returnvalue_2 (UserInterface|CreateWidget "/Game/Ewan/UI/WB_Red.WB_Red_C" (Game|GetPlayerController 0)))
    (UserInterface|Viewport|AddtoViewport _returnvalue_2 0)
    (Utilities|FlowControl|Delay 3.0)
    (Default|Respawn _asbp_gab_perso)
    (Variables|Default|SetIsSeeing false)
    (bind _foundwidgets (Widget|GetAllWidgetsOfClass "/Game/Ewan/UI/WB_Red.WB_Red_C" true))
    (for _array_element _foundwidgets
      (Widget|RemovefromParent _array_element)
      (Variables|/Script/Engine.CharacterMovementComponent|SetMaxWalkSpeed (Variables|/Script/Engine.Character|GetCharacterMovement _asbp_gab_perso) 5e+02))))

(event Custom|VentCheck
  (bind _returnvalue (Game|GetPlayerCharacter 0))
  (bind _asbp_gab_perso (Utilities|Casting|CastToBP_GabPerso _returnvalue))
  (if (Variables|/Game/Gabriel/BP_GabPerso.BP_GabPerso_C|GetInVent? _asbp_gab_perso)
    (Default|Respawn _asbp_gab_perso)))

(event EventBeginPlay
  (bind _spotlight (Variables|Default|GetSpotLight))
  (bind _visionangle (Variables|Default|GetVisionAngle))
  (Rendering|Lighting|SetInnerConeAngle _spotlight _visionangle)
  (Rendering|Lighting|SetOuterConeAngle _spotlight (+ _visionangle 3.0))
  (Class|PawnSensingComponent|SetPeripheralVisionAngle (Variables|Default|GetPawnSensing) _visionangle))

(fn ConstructionScript)