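; BP_AICharacter2 is a guard AI character that sends the player back to respawn when it spots them.
; On BeginPlay, a shared VisionAngle sets both the spotlight cone and the PawnSensing peripheral angle, so the light mirrors the detection area.
; Seeing the player pawn calls Respawn on BP_CharacterEwan.
; Tick prints a Visible or Hidden debug string from IsSeeing, which clears immediately after the respawn call.
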(event OnSeePawn(PawnSensing)
  (params (Pawn :type Pawn%20Object%20Reference))
  (bind _returnvalue (Game|Player|GetPlayerPawn 0))
  (if (== Pawn _returnvalue)
    (Variables|Default|SetIsSeeing true)
    (bind _asbp_character_ewan (Utilities|Casting|CastToBP_CharacterEwan _returnvalue))
    (Default|Respawn _asbp_character_ewan)
    (Variables|Default|SetIsSeeing false)))

(event EventBeginPlay
  (bind _visionangle (Variables|Default|GetVisionAngle))
  (bind _spotlight (Variables|Default|GetSpotLight))
  (Rendering|Lighting|SetInnerConeAngle _spotlight _visionangle)
  (Rendering|Lighting|SetOuterConeAngle _spotlight (+ _visionangle 3.0))
  (Class|PawnSensingComponent|SetPeripheralVisionAngle (Variables|Default|GetPawnSensing) _visionangle))

(event EventTick
  (params (DeltaSeconds :type Float%20%28single-precision%29))
  (if (Variables|Default|GetIsSeeing)
    (Development|PrintString "Visible")
    (else
      (Development|PrintString "Hidden"))))

(fn ConstructionScript)