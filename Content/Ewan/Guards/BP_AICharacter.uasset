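; BP_AICharacter is a guard AI character that detects pawns within a vision cone.
; On BeginPlay, VisionAngle sets both the SpotLight cone and the PawnSensing peripheral vision angle, so the light shows the guard's field of view.
; Each sighting sets IsSeeing, and a retriggerable delay clears it shortly after sightings stop.
; Tick prints Visible or Hidden from that flag as debug feedback.
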(event OnSeePawn(PawnSensing)
  (params (Pawn :type Pawn%20Object%20Reference))
  (Variables|Default|SetIsSeeing true)
  (Utilities|FlowControl|RetriggerableDelay 0.6)
  (Variables|Default|SetIsSeeing false))

(event EventBeginPlay
  (bind _spotlight (Variables|Default|GetSpotLight))
  (bind _visionangle (Variables|Default|GetVisionAngle))
  (Rendering|Lighting|SetInnerConeAngle _spotlight _visionangle)
  (Rendering|Lighting|SetOuterConeAngle _spotlight (+ _visionangle 3.0))
  (Class|PawnSensingComponent|SetPeripheralVisionAngle (Variables|Default|GetPawnSensing) _visionangle))

(event Collision|EventActorBeginOverlap
  (params (OtherActor :type Actor%20Object%20Reference)))

(event EventTick
  (params (DeltaSeconds :type Float%20%28single-precision%29))
  (if (Variables|Default|GetIsSeeing)
    (Development|PrintString "Visible")
    (else
      (Development|PrintString "Hidden"))))

(fn ConstructionScript)